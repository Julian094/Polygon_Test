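; Trigger actor that opens a character and animation change UI when the first-person character enters its box.
; On overlap it turns the player relative to its yaw, aligns their world Y to its own and creates WBP_ChangeCharacterAnimation.
; It then disables player movement and switches to UI-only input with a mouse cursor.
; Interface events swap its skeletal mesh and play montages on it.
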(event `self.Box.OnComponentBeginOverlap`
  (params (OverlappedComponent :type "PrimitiveComponent Object Reference") (OtherActor :type "Actor Object Reference") (OtherComp :type "PrimitiveComponent Object Reference") (OtherBodyIndex :type Integer) (bFromSweep :type Boolean) (SweepResult :type "HitResult Structure (by ref)"))
  (bind (_returnvalue_roll _returnvalue_pitch _returnvalue_yaw) (`KismetMathLibrary.BreakRotator` (`self.K2_GetActorRotation`)))
  ;[1 1 1] Begin Overlap
  (bind _asbp_first_person_character (cast `/Game/FirstPerson/Blueprints/BP_FirstPersonCharacter` OtherActor))
  (`Controller.SetControlRotation` (`Pawn.GetController` _asbp_first_person_character) (`KismetMathLibrary.MakeRotator` 0.0 0.0 (+ _returnvalue_yaw -90.0)))
  (`self.SetActorLocation` _asbp_first_person_character)
  (bind _returnvalue (`|CreateWidget` "/Game/Blueprints/ActiavteAnimations/WBP_ChangeCharacterAnimation.WBP_ChangeCharacterAnimation_C" null self (`self.SkeletalMesh_0`)))
  (`UserWidget.AddToViewport` _returnvalue 0)
  (`self.F_SetUIGameMode` _returnvalue))

(event `/Game/Blueprints/Interfaces/BPI_ChangeCharacter.BPI_ChangeSkeletalMesh`
  (params (NewMesh :type "SkeletalMesh Object Reference"))
  ;[1 1 1] Function called from BPI
  (`SkeletalMeshComponent.SetSkeletalMeshAsset` (`self.SkeletalMesh`) NewMesh))

(event `/Game/Blueprints/Interfaces/BPI_ChangeCharacter.BPI_PlayAnimation`
  (params (AnimMontage :type "AnimMontage Object Reference"))
  ;[1 1 1] Function called from BPI
  (`|PlayMontage` (`self.SkeletalMesh`) AnimMontage))

(fn `F_SetUIGameMode`
  (params (InWidgetToFocus :type "Widget Object Reference"))
  (bind _returnvalue (`GameplayStatics.GetPlayerCharacter` 0))
  (`CharacterMovementComponent.SetMovementMode` (`Character.CharacterMovement` _returnvalue) "MOVE_None" 0)
  (bind _asplayer_controller (cast `PlayerController` (`self.GetOwner` _returnvalue)))
  (`WidgetBlueprintLibrary.SetInputMode_UIOnlyEx` _asplayer_controller InWidgetToFocus)
  (set `PlayerController.bShowMouseCursor` true _asplayer_controller))

(fn `SetActorLocation`
  (params (RefCharacter :type "Actor Object Reference"))
  (bind (_returnvalue_x _returnvalue_y) (`KismetMathLibrary.BreakVector` (`self.K2_GetActorLocation`)))
  (bind (_returnvalue_x_2 _returnvalue_y_2 _returnvalue_z) (`KismetMathLibrary.BreakVector` (`self.K2_GetActorLocation` RefCharacter)))
  (`self.K2_SetActorLocation` RefCharacter (`KismetMathLibrary.MakeVector` _returnvalue_x_2 _returnvalue_y _returnvalue_z) false false))

(fn `UserConstructionScript`)