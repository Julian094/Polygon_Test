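; Teleport actor Blueprint that lets the player choose a destination portal and plays a visual effect around the jump.
; StarInteraction, called from C++, opens WBP_SelectMainTeleport with the target point names and switches to UI-only input with a visible cursor.
; StartEffect drives VisualEffect through a timeline, then calls Teleport on the chosen portal when it finishes.
; SetInitialVisualEffect runs a second timeline in reverse to restore the effect's initial value.
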(event `self.BP_StarInteraction`
  ;[1 1 1] Event called from c++, create widget for interacting
  (bind _returnvalue (`|CreateWidget` "/Game/Blueprints/Teleport/WBP_SelectMainTeleport.WBP_SelectMainTeleport_C" null self (`self.TargetsPointsNames`)))
  (`UserWidget.AddToViewport` _returnvalue 0)
  (`self.F_SetUIGameMode` _returnvalue))

(event `StartEffect`
  (params (ObjectivePortal :type "Actor Object Reference"))
  ;[1 1 1] Timeline for setting up value of visual effect
  (bind (_direction _newtrack_0) (`Timeline|Timeline` :!via `PlayFromStart`)
    (:`Update`
      (`self.VisualEffect` (`KismetMathLibrary.Lerp` 1.2 0.0 _newtrack_0)))
    (:`Finished`
      (`self.Teleport` ObjectivePortal))))

(event `self.BP_SetInitialVisualEffect`
  ;[1 1 1] Timeline for setting up intial value of visual effect
  (bind (_direction _newtrack_0) (`Timeline|Timeline_0` :!via `ReverseFromEnd`)
    (:`Update`
      (`self.VisualEffect` (`KismetMathLibrary.Lerp` 1.2 0.0 _newtrack_0)))))

(fn `F_SetUIGameMode`
  (params (InWidgetToFocus :type "Widget Object Reference"))
  (bind _asplayer_controller (cast `PlayerController` (`self.GetOwner` (`GameplayStatics.GetPlayerCharacter` 0))))
  (`WidgetBlueprintLibrary.SetInputMode_UIOnlyEx` _asplayer_controller InWidgetToFocus)
  (set `PlayerController.bShowMouseCursor` true _asplayer_controller))

(fn `UserConstructionScript`)