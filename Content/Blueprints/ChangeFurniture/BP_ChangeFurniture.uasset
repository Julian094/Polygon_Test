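; BP_ChangeFurniture is an interactable that opens a mesh selection menu for changing either walls or furniture.
; On StartInteraction, it removes a valid interaction widget, then picks the Walls or Furnitures map based on IsChangingWall.
; CreateWidget splits that map into meshes and names, passes them with a self reference to WBP_SelectMeshes, and adds it to the viewport.
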(event `self.BP_StartInteraction`
  (bind _widgetinteractionclass (`self.WidgetInteractionClass`)
    (:`then`
      (`Widget.RemoveFromParent` _widgetinteractionclass)
      (switch `int` (`KismetMathLibrary.SelectInt` 1 0 (`self.bIsChangingWall`))
        (:`0`
          (`self.CreateWidget` (`self.Furnitures`)))
        (:`1`
          (`self.CreateWidget` (`self.Walls`)))))
    (:`else`)))

(fn `CreateWidget`
  (params (TargetMap :type "Map of StaticMesh Object Reference to Name (by ref)"))
  (bind _keys (`BlueprintMapLibrary.Map_Keys` TargetMap))
  (bind _values (`BlueprintMapLibrary.Map_Values` TargetMap))
  (bind _returnvalue (`|CreateWidget` "/Game/Blueprints/ChangeFurniture/WBP_SelectMeshes.WBP_SelectMeshes_C" null self _keys _values))
  (`UserWidget.AddToViewport` _returnvalue 0))

(fn `UserConstructionScript`)